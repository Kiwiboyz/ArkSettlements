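; Dodo character Blueprint for Ark Settlements that can dress the dodo as a "Dodo Bunny".
; On BeginPlay it checks the ShooterGameState's active event, in what appears to be a seasonal event switch.
; The costume path adds a bunny-ears static mesh at runtime, attaches it to the head socket, and overrides the drag weight and descriptive name.
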(event `self.ReceiveBeginPlay`
  (`parent.ReceiveBeginPlay`)
  (bind _asshootergamestate (cast `ShooterGameState` (`GameplayStatics.GetGameState`)))
  (switch `name` (`ShooterGameState.ActiveEvent` _asshootergamestate)
    (:`Easter`
      (bind _returnvalue (`AddComponent|StaticMeshComponent_26` :`bManualAttachment` true :`RelativeTransform` (`KismetMathLibrary.MakeTransform` (1.047986 2.302929 0.061898) (struct :`Pitch` -90.0 :`Roll` -89.999969) (0.8 0.7 0.8))))
      (`StaticMeshComponent.SetStaticMesh` _returnvalue "/Game/PrimalEarth/Human/Male/Outfits/Easter/BunnyEars/SM_BunnyEars.SM_BunnyEars")
      (`SceneComponent.K2_AttachTo` _returnvalue (`self.Mesh`) "c_head" "KeepRelativeOffset" true)
      (set `self.DragWeight` 500.0)
      (set `self.DescriptiveName` "Dodo Bunny"))))

(fn `UserConstructionScript`
  (`parent.UserConstructionScript`))